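; Player-controlled tank pawn Blueprint that wires its parts together and routes input to them.
; On BeginPlay it hands the barrel and turret to the TankAiming component and both tracks to TankMovement.
; Movement axes go to TankMovement as drive and turn intents, and Fire calls TankAiming.
; Aim axes rotate a separate azimuth gimbal and spring arm, scaled by frame delta time, for yaw and pitch.
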(event EventBeginPlay
  (Class|TankAimingComponent|Initialise (Variables|Default|GetTankAiming) (Variables|Default|GetTankBarrel) (Variables|Default|GetTankTurret))
  (Class|TankMovementComponent|Initialise (Variables|Default|GetTankMovement) (Variables|Default|GetLeft%20TankTrack) (Variables|Default|GetRight%20TankTrack)))

(event Input|ActionEvents|InputActionFire
  (params (Key :type Key%20Structure :default "AnyKey"))
  ;[1 1 1] Ballistics Input
  (:Pressed
    (Class|TankAimingComponent|Fire (Variables|Default|GetTankAiming))))

(event Input|AxisEvents|InputAxisAimAzimuth
  (params (AxisValue :type Float%20%28single-precision%29))
  ;[1 1 1] Azimuth X-Axis Rotation
  (Transformation|AddLocalRotation (Variables|Default|GetAzimuth%20Gimbal) (Math|Rotator|MakeRotator 0.0 0.0 (* AxisValue (Utilities|Time|GetWorldDeltaSeconds) 1e+02)) false false))

(event Input|AxisEvents|InputAxisIntendTurnRight
  (params (AxisValue :type Float%20%28single-precision%29))
  ;[1 1 1] Track Control
  (Class|TankMovementComponent|IntendTurnRight (Variables|Default|GetTankMovement) AxisValue))

(event Input|AxisEvents|InputAxisIntendMovementForward
  (params (AxisValue :type Float%20%28single-precision%29))
  ;[1 1 1] Track Control
  (Class|TankMovementComponent|IntendMoveForward (Variables|Default|GetTankMovement) AxisValue))

(event Input|AxisEvents|InputAxisAimElevation
  (params (AxisValue :type Float%20%28single-precision%29))
  ;[1 1 1] Elevation Y-Axis Rotation
  (Transformation|AddLocalRotation (Variables|Default|GetSpringArm) (Math|Rotator|MakeRotator 0.0 (* AxisValue (Utilities|Time|GetWorldDeltaSeconds) 1e+02) 0.0) false false))

(fn ConstructionScript)